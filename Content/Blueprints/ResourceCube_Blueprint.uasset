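; Destructible wood resource cube that loses health when hit by first-person projectiles and shows its health as inspect text.
; Hit validates the projectile, gets its firing player, then destroys the projectile.
; Non-lethal hits play a small explosion and spawn another cube at a random location from the player's RandomLocationWithinWorld.
; The lethal hit explodes bigger, destroys the cube, awards wood and optionally spawns a replacement.
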(event EventBeginPlay
  (Variables|/Script/Engine.ActorComponent|SetComponentTags (Variables|Debug|GetStaticMeshComponent) (Utilities|Array|MakeArray "Inspectable")))

(event Collision|EventActorBeginOverlap
  (params (OtherActor :type Actor%20Object%20Reference)))

(event EventTick
  (params (DeltaSeconds :type Float%20%28single-precision%29)))

(event Collision|EventHit
  (params (MyComp :type Primitive%20Component%20Object%20Reference) (Other :type Actor%20Object%20Reference) (OtherComp :type Primitive%20Component%20Object%20Reference) (bSelfMoved :type Boolean) (HitLocation :type Vector :default "0, 0, 0") (HitNormal :type Vector :default "0, 0, 0") (NormalImpulse :type Vector :default "0, 0, 0") (Hit :type Hit%20Result%20Structure%20%28by%20ref%29))
  (bind (_projectile _firing_player _success_) (CallFunction|HitbyFirstPersonProjectile? Other))
  (if _success_
    (Utilities|FlowControl|Sequence
      (:then_0
        (bind _output_get (Variables|Default|SetHealth (- (Variables|Default|GetHealth) 25)))
        (Math|Integer|CompareInt _output_get
          (:>
            (Audio|PlaySoundatLocation "/Game/StarterContent/Audio/Explosion02.Explosion02" HitLocation "0, 0, 0" 0.25 1.0 0.0 0 0 0)
            (Effects|SpawnEmitterAttached "/Game/StarterContent/Particles/P_Explosion.P_Explosion" MyComp "None" "0, 0, 0" "0, 0, 0" "0.500000,0.500000,0.500000")
            (CallFunction|SpawnNewWithinArena _firing_player))
          (:==
            (if (== _firing_player 0) :!label _label
              (Development|PrintString "Player was null??")
              (else
                (Audio|PlaySoundatLocation "/Game/StarterContent/Audio/Explosion01.Explosion01" HitLocation "0, 0, 0" 1.0 1.0 0.0 0 0 0)
                (Actor|DestroyActor)
                (Effects|SpawnEmitteratLocation "/Game/StarterContent/Particles/P_Explosion.P_Explosion" HitLocation "0, 0, 0" "2.500000,2.500000,2.500000")
                (Default|AddWood _firing_player (Variables|Default|GetWood%20Value))
                (if (Variables|Default|GetSpawn%20New%20Resources%20within%20Arena?)
                  (CallFunction|SpawnNewWithinArena _firing_player)))))
          (:<
            (goto _label))))
      (:then_1
        (Actor|DestroyActor _projectile) ; Garbage collection to match prev behaviour
      ))))

(fn ConstructionScript)

(fn HitbyFirstPersonProjectile?
  (params (Event%20Hit%20Other%20Actor :type Actor%20Object%20Reference))
  (if (== (Utilities|GetClass Event%20Hit%20Other%20Actor) "/Game/FirstPersonBP/Blueprints/FirstPersonProjectile.FirstPersonProjectile_C")
    (bind _asfirst_person_projectile (Utilities|Casting|CastToFirstPersonProjectile Event%20Hit%20Other%20Actor)
      (:then
        (bind _output_get (LocalVariables|SetNewLocalVar_0 (Variables|/Game/FirstPersonBP/Blueprints/FirstPersonProjectile.FirstPersonProjectile_C|GetFiring%20Player _asfirst_person_projectile)))
        (return _asfirst_person_projectile _output_get true))
      (:CastFailed
        (Development|PrintString (Utilities|String|BuildString(Object) "Expected FirstPersonProjectile, got" "" Event%20Hit%20Other%20Actor))
        (return 0 0 false)))
    (else
      (return 0 0 false))))

(fn SpawnNewWithinArena
  (params (FirstPersonCharacter :type First%20Person%20Character%20Object%20Reference%20%28by%20ref%29))
  (bind _location (Default|RandomLocationWithinWorld FirstPersonCharacter))
  (bind _returnvalue (Game|SpawnActorfromClass (Utilities|GetClass self) (Math|Transform|MakeTransform _location (Math|Random|RandomRotator false)) "Undefined" 0 0))
  (Development|PrintString (Utilities|String|BuildString(Vector) "" "Created new box at" (Transformation|GetActorLocation _returnvalue))))

(fn InspectText
  (return (Utilities|Text|ToText(String) (Utilities|String|BuildString(Integer) "" "Wood (" (Variables|Default|GetHealth) " hp)"))))