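; ValueControlsScreen is an in-world screen actor that holds an adjustable value and displays it as "x=" text.
; IncrementValue adds a delta to the value and refreshes ValueRender, while GetInspectText returns the stored inspect text.
; Each tick, HighlightSphere's material opacity is lerped by player distance relative to 1.5 times the FirstPersonCharacter's PickUpDistance, so the highlight strengthens as the player approaches.
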(event EventBeginPlay
  (Rendering|Material|SetScalarParameterValueonMaterials (Variables|Default|GetHighlightSphere) "Opacity" 0.0))

(event Collision|EventActorBeginOverlap
  (params (OtherActor :type Actor%20Object%20Reference)))

(event EventTick
  (params (DeltaSeconds :type Float%20%28single-precision%29))
  (bind _returnvalue (Game|Player|GetPlayerPawn 0))
  (bind _asfirst_person_character (Utilities|Casting|CastToFirstPersonCharacter _returnvalue))
  (Rendering|Material|SetScalarParameterValueonMaterials (Variables|Default|GetHighlightSphere) "Opacity" (Math|Float|Lerp 1.0 0.0 (/ (Math|Vector|Distance(Vector) (Transformation|GetWorldLocation (Variables|Default|GetDefaultSceneRoot)) (Transformation|GetActorLocation _returnvalue)) (* (Variables|/Game/FirstPersonBP/Blueprints/FirstPersonCharacter.FirstPersonCharacter_C|GetPick%20Up%20Distance _asfirst_person_character) 1.5)))))

(fn ConstructionScript)

(fn IncrementValue
  (params (Delta :type Integer))
  (bind _output_get (Variables|Default|SetValue (+ (Variables|Default|GetValue) Delta)))
  (Rendering|Components|TextRender|SetText (Variables|Default|GetValueRender) (Utilities|Text|ToText(String) (Utilities|String|BuildString(Integer) "x=" "" _output_get))))

(fn GetInspectText
  (return (Variables|Default|GetInspect%20Text)))